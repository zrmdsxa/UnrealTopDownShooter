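; Player controller for a top-down shooter that handles world-axis movement, cursor aiming, firing and reloading for the TopDownCharacter.
; Pressing Fire snaps the pawn toward the cursor and opens a gate that updates LookAngle each tick.
; While shooting, Tick spawns delay-throttled bullets from the weapon's arrow and drains its Loader.
; Reload blocks movement during a timed refill; GetParameters exposes aim and reload state, while the FlipPlayer check is unwired.
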(event Custom|StartFire1
  (if (> (Variables|/Game/TopDownBP/Blueprints/TopDownCharacter.TopDownCharacter_C|GetHealth (Variables|Default|GetCharacterReference)) 0.0)
    (Variables|/Script/Engine.CharacterMovementComponent|SetbOrientRotationToMovement (Variables|/Script/Engine.Character|GetCharacterMovement (Variables|Default|GetCharacterReference)) false)
    (Variables|Default|SetisShooting true)
    (CallFunction|RotatetoAim)))

(event Custom|StopFire1
  (Variables|/Script/Engine.CharacterMovementComponent|SetbOrientRotationToMovement (Variables|/Script/Engine.Character|GetCharacterMovement (Variables|Default|GetCharacterReference)) true)
  (Variables|Default|SetisShooting false))

(event Custom|Reloaded
  ;[1 1 1] Finish reload
  (bind _output_get (Variables|Default|SetisReloading false))
  (Input|SetIgnoreMoveInput _output_get)
  (Components|Animation|SetAnimationMode (Variables|/Script/Engine.Character|GetMesh (Variables|Default|GetCharacterReference)) "AnimationBlueprint"))

(event Custom|OutOfAmmo
  ;[1 1 1] Reload
  (if (> (Variables|/Game/TopDownBP/Blueprints/TopDownCharacter.TopDownCharacter_C|GetHealth (Variables|Default|GetCharacterReference)) 0.0)
    (if (not (Variables|Default|GetisReloading))
      (bind _output_get (Variables|Default|SetisReloading true))
      (Input|SetIgnoreMoveInput _output_get)
      (Utilities|FlowControl|Delay 2.0)
      (if (> (Variables|/Game/TopDownBP/Blueprints/TopDownCharacter.TopDownCharacter_C|GetHealth (Variables|Default|GetCharacterReference)) 0.0)
        (Default|TopUpWeapon (Variables|/Game/TopDownBP/Blueprints/TopDownCharacter.TopDownCharacter_C|GetWeaponEquipped (Variables|Default|GetCharacterReference)))
        (CallFunction|Reloaded)))))

(event EventBeginPlay
  (bind _astop_down_character (Utilities|Casting|CastToTopDownCharacter (Pawn|GetControlledPawn)))
  (Variables|Default|SetCharacterReference _astop_down_character))

(event EventTick
  (params (DeltaSeconds :type Float%20%28single-precision%29))
  (bind _characterreference (Variables|Default|GetCharacterReference))
  (bind _weaponequipped (Variables|/Game/TopDownBP/Blueprints/TopDownCharacter.TopDownCharacter_C|GetWeaponEquipped _characterreference))
  (if (> (Variables|/Game/TopDownBP/Blueprints/TopDownCharacter.TopDownCharacter_C|GetHealth (Variables|Default|GetCharacterReference)) 0.0)
    (Utilities|FlowControl|Sequence
      (:then_0
        (Utilities|FlowControl|Gate true
          (:Exit
            (CallFunction|SetAimAngle))))
      (:then_1
        (if (Variables|Default|GetisShooting)
          (if (> (Variables|/Game/mystuff/blueprints/weapon.weapon_C|GetLoader _weaponequipped) 0.0)
            (if (not (Variables|Default|GetisReloading))
              (Utilities|FlowControl|Delay 0.1)
              (bind _returnvalue (Game|SpawnActorfromClass "/Game/mystuff/blueprints/Bullet.Bullet_C" (Transformation|GetWorldTransform (Variables|/Game/mystuff/blueprints/weapon.weapon_C|GetArrow _weaponequipped)) "Undefined" 0 0))
              (Transformation|SetWorldScale3D (Variables|/Game/mystuff/blueprints/Bullet.Bullet_C|GetSphere _returnvalue) "0.100000,0.100000,0.100000")
              (Variables|/Game/mystuff/blueprints/weapon.weapon_C|SetLoader _weaponequipped (- (Variables|/Game/mystuff/blueprints/weapon.weapon_C|GetLoader _weaponequipped) 1.0)))))))))

(event Input|ActionEvents|InputActionFire
  (params (Key :type Key%20Structure :default "AnyKey"))
  (bind _characterreference (Variables|Default|GetCharacterReference))
  (bind _weaponequipped (Variables|/Game/TopDownBP/Blueprints/TopDownCharacter.TopDownCharacter_C|GetWeaponEquipped _characterreference))
  (:Pressed
    (Utilities|IsValid _weaponequipped
      (:Is%20Valid
        (CallFunction|StartFire1)
        (Utilities|FlowControl|Gate true) ; enters at Open
      )))
  (:Released
    (Utilities|IsValid _weaponequipped
      (:Is%20Valid
        (CallFunction|StopFire1)
        (Utilities|FlowControl|Gate true) ; enters at Close
      ))))

(event Input|ActionEvents|InputActionReload
  (params (Key :type Key%20Structure :default "AnyKey"))
  ;[1 1 1] Reload
  (:Pressed
    (CallFunction|OutOfAmmo)))

(event Input|AxisEvents|InputAxisMoveRight
  (params (AxisValue :type Float%20%28single-precision%29))
  ;[1 1 1] movement inputs
  (Pawn|Input|AddMovementInput (Game|Player|GetPlayerPawn 0) (Math|Vector|MakeVector 0.0 1.0 0.0) AxisValue false))

(event Input|AxisEvents|InputAxisMoveForward
  (params (AxisValue :type Float%20%28single-precision%29))
  ;[1 1 1] movement inputs
  (Pawn|Input|AddMovementInput (Game|Player|GetPlayerPawn 0) (Math|Vector|MakeVector 1.0 0.0 0.0) AxisValue false))

(fn ConstructionScript)

(fn RotatetoAim
  (bind _returnvalue (Pawn|GetControlledPawn))
  (Transformation|SetActorRotation _returnvalue (Math|Rotator|MakeRotator 0.0 0.0 (.Yaw (Math|Rotator|BreakRotator (Math|Rotator|FindLookatRotation (Transformation|GetActorLocation _returnvalue) (.Location (Collision|BreakHitResult (.HitResult (Game|Player|GetHitResultUnderCursorbyChannel "TraceTypeQuery1" true))))))))))

(fn SetAimAngle
  (bind _returnvalue (Pawn|GetControlledPawn))
  (Variables|Default|SetLookAngle (- (.Yaw (Math|Rotator|BreakRotator (Math|Rotator|FindLookatRotation (Transformation|GetActorLocation _returnvalue) (.Location (Collision|BreakHitResult (.HitResult (Game|Player|GetHitResultUnderCursorbyChannel "TraceTypeQuery1" true))))))) (.Yaw (Math|Rotator|BreakRotator (Transformation|GetActorRotation _returnvalue))))))

(fn FlipPlayer
  (bind _returnvalue (Pawn|GetControlledPawn))
  (bind _returnvalue_2 (Transformation|GetActorRotation _returnvalue))
  (bind _returnvalue_3 (Math|Rotator|GetRotationXVector _returnvalue_2))
  (bind _returnvalue_4 (Math|Vector|RotateVector _returnvalue_3 "0,180.000000, 0"))
  (if (> (.Z (Math|Vector|BreakVector _returnvalue_4)) 1.8e+02)
    (Transformation|SetActorRotation _returnvalue (Math|Conversions|RotationFromXVector _returnvalue_4))
    (else
      (Transformation|SetActorRotation _returnvalue (Math|Conversions|RotationFromXVector (Math|Vector|RotateVector _returnvalue_4 "0,-360.000000, 0"))))))

(fn GetParameters
  (return (Variables|Default|GetisShooting) (Variables|Default|GetLookAngle) (Variables|Default|GetisReloading)))

(fn SetAnimReference
  (params (animbp :type Anim%20BP%20Object%20Reference))
  (Variables|Default|SetanimRef animbp))