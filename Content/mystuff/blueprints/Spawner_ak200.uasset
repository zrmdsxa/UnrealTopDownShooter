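; Weapon spawner actor that keeps one pickup from its Spawnable class list present at its Arrow component.
; A looping three-second timer started on BeginPlay calls SpawnObject, which spawns a random class from the list only while ObjectExist is false.
; The spawned actor is cast to weapon_ak200 and given a reference back to the spawner; the flag is set only if that cast succeeds.
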(event Custom|SpawnObject
  (bind _spawnable (Variables|Default|GetSpawnable))
  (if (not (Variables|Default|GetObjectExist))
    (bind _returnvalue (Game|SpawnActorfromClass (Utilities|Array|Get(acopy) _spawnable (Math|Random|RandomInteger (Utilities|Array|Length _spawnable))) (Transformation|GetWorldTransform (Variables|Default|GetArrow)) "Undefined" 0 0))
    (bind _asweapon_ak_200 (Utilities|Casting|CastToweapon_ak200 _returnvalue))
    (Variables|/Game/mystuff/blueprints/weapon_ak200.weapon_ak200_C|Setspawner_ref _asweapon_ak_200 self)
    (Variables|Default|SetObjectExist true)))

(event EventBeginPlay
  (Utilities|Time|SetTimerbyFunctionName 0 "SpawnObject" 3.0 true))

(event Collision|EventActorBeginOverlap
  (params (OtherActor :type Actor%20Object%20Reference)))

(event EventTick
  (params (DeltaSeconds :type Float%20%28single-precision%29)))

(fn ConstructionScript)