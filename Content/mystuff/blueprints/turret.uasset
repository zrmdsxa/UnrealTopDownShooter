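; Turret actor that detects when the player character comes within firing range.
; Every tick it casts the first player controller to myPlayerController and measures the distance from its static mesh to the referenced character's capsule.
; Within the fixed radius it only prints a "fire" debug string, with no aiming, projectile or damage logic.
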(event EventBeginPlay)

(event Collision|EventActorBeginOverlap
  (params (OtherActor :type Actor%20Object%20Reference)))

(event EventTick
  (params (DeltaSeconds :type Float%20%28single-precision%29))
  (bind _asmy_player_controller (Utilities|Casting|CastTomyPlayerController (Game|GetPlayerController 0)))
  (if (<= (Math|Vector|VectorLength (- (.Location (Math|Transform|BreakTransform (Transformation|GetWorldTransform (Variables|/Script/Engine.Character|GetCapsuleComponent (Variables|/Game/mystuff/blueprints/myPlayerController.myPlayerController_C|GetCharacterReference _asmy_player_controller))))) (.Location (Math|Transform|BreakTransform (Transformation|GetWorldTransform (Variables|Debug|GetStaticMeshComponent self)))))) 1e+03)
    (Development|PrintString "fire")))

(fn ConstructionScript)