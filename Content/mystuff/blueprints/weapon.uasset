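; Pickup weapon actor that a TopDownCharacter collects on overlap and fires as a projectile gun.
; On collection it attaches to the player mesh's back socket, stops rotating and resets its spawner component.
; StartFire and StopFire control a looping timer that spends ammo and spawns small bullets at the arrow.
; When empty it either destroys itself or signals out-of-ammo to the player controller until TopUpWeapon refills it.
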(event Custom|StartFire
  (Utilities|Time|SetTimerbyFunctionName 0 "Fire" (Variables|Default|GetFireRate) true))

(event Custom|StopFire
  (Utilities|Time|ClearTimerbyFunctionName 0 "Fire"))

(event Custom|TopUp%20Weapon
  (Variables|Default|SetLoader (Variables|Default|GetMaxAmmo))
  (Variables|Default|SetisReloading false))

(event EventBeginPlay)

(event Collision|EventActorBeginOverlap
  (params (OtherActor :type Actor%20Object%20Reference))
  ;[1 1 1] Player touch weapon
  (bind _astop_down_character (Utilities|Casting|CastToTopDownCharacter OtherActor))
  (bind _result (Default|Collect _astop_down_character self))
  (if _result
    (Transformation|AttachComponentToComponent (Variables|/Script/Engine.Character|GetMesh (Game|GetPlayerCharacter 0)) "WeaponBack" "SnapToTarget" "SnapToTarget" "SnapToTarget" true)
    (Components|Activation|Deactivate (Variables|Default|GetRotatingMovement))
    ;[1 1 1] Comment
    (Default|ResetSpawner (Actor|GetComponentsByClass "/Game/mystuff/blueprints/SpawnerComponent.SpawnerComponent_C"))))

(event EventTick
  (params (DeltaSeconds :type Float%20%28single-precision%29)))

(fn ConstructionScript)

(fn Fire
  (if (and (not (Variables|Default|GetisReloading)) (> (Variables|Default|GetLoader) 0.0))
    (Variables|Default|SetLoader (- (Variables|Default|GetLoader) 1.0))
    (bind _returnvalue (Game|SpawnActorfromClass "/Game/mystuff/blueprints/Bullet.Bullet_C" (Transformation|GetSocketTransform (Variables|Default|GetArrow) "None" "RTS_World") "Undefined" 0 0))
    (Transformation|SetWorldScale3D (Variables|/Game/mystuff/blueprints/Bullet.Bullet_C|GetSphere _returnvalue) "0.100000,0.100000,0.100000")
    (elif (Variables|Default|GetselfDestroy)
      (CallFunction|DestroyIt)
      (else
        (Variables|Default|SetisReloading true)
        (bind _asmy_player_controller (Utilities|Casting|CastTomyPlayerController (Game|GetPlayerController 0)))
        (Default|OutOfAmmo _asmy_player_controller)))))

(fn DestroyIt
  (Actor|DestroyActor)
  (bind _asmy_player_controller (Utilities|Casting|CastTomyPlayerController (Game|GetPlayerController 0)))
  (Default|StopFire1 _asmy_player_controller))