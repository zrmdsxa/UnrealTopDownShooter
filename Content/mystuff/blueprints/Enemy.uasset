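; Enemy actor for a top-down game that takes bullet hits and damages the player character on contact.
; Overlapping a Bullet subtracts a fixed amount of Health, and the enemy dies when Health reaches zero.
; Its Sphere component detects the TopDownCharacter, applies Strength as damage, then kills the enemy immediately.
; Both death paths share one branch that spawns an ExplodePS actor at the enemy's transform and destroys it.
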(event OnComponentBeginOverlap(Sphere)
  (params (OverlappedComponent :type Primitive%20Component%20Object%20Reference) (OtherActor :type Actor%20Object%20Reference) (OtherComp :type Primitive%20Component%20Object%20Reference) (OtherBodyIndex :type Integer) (bFromSweep :type Boolean) (SweepResult :type Hit%20Result%20Structure%20%28by%20ref%29))
  (bind _astop_down_character (Utilities|Casting|CastToTopDownCharacter OtherActor))
  (Default|TakeDamage _astop_down_character (Variables|Default|Getstrength))
  (Game|SpawnActorfromClass "/Game/mystuff/blueprints/explodePS.explodePS_C" (Transformation|GetActorTransform self) "Undefined" 0 0)
  (Actor|DestroyActor))

(event EventBeginPlay)

(event Collision|EventActorBeginOverlap
  (params (OtherActor :type Actor%20Object%20Reference))
  ;[1 1 1] hitbybullet
  (Utilities|Casting|CastToBullet OtherActor)
  (bind _output_get (Variables|Default|Sethealth (- (Variables|Default|Gethealth) 1e+01)))
  (if (<= _output_get 0.0)
    (Game|SpawnActorfromClass "/Game/mystuff/blueprints/explodePS.explodePS_C" (Transformation|GetActorTransform self) "Undefined" 0 0)
    (Actor|DestroyActor)))

(event EventTick
  (params (DeltaSeconds :type Float%20%28single-precision%29)))

(fn ConstructionScript)