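; M249 weapon pickup, a child Blueprint that sets its own ammo capacity, loader size and fire rate on BeginPlay.
; On overlap it runs the parent logic, then asks the overlapping TopDownCharacter to collect it.
; If collected, it clears its spawner's ObjectExist flag, snaps to the WeaponBack socket on player 0's mesh rather than the overlapping character's, and stops its rotating movement.
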(event EventBeginPlay
  (Variables|Default|SetMaxAmmo 2e+02)
  (Variables|Default|SetLoader 2e+02)
  (Variables|Default|SetFireRate 0.05))

(event Collision|EventActorBeginOverlap
  (params (OtherActor :type Actor%20Object%20Reference))
  (|CallParentFunction OtherActor)
  (bind _astop_down_character (Utilities|Casting|CastToTopDownCharacter OtherActor))
  (bind _result (Default|Collect _astop_down_character self))
  (if _result
    (Variables|/Game/mystuff/blueprints/Spawner_m249.Spawner_m249_C|SetObjectExist (Variables|Default|Getspawner_ref) false)
    (Transformation|AttachComponentToComponent (Variables|/Script/Engine.Character|GetMesh (Game|GetPlayerCharacter 0)) "WeaponBack" "SnapToTarget" "SnapToTarget" "SnapToTarget" true)
    (Components|Activation|Deactivate (Variables|Default|GetRotatingMovement))))

(event EventTick
  (params (DeltaSeconds :type Float%20%28single-precision%29)))

(fn ConstructionScript
  (|CallParentFunction))